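; BP_AK4 is a pickup rifle that attaches to the first-person character and can fire.
; Overlapping its Box with BP_FirstPersonCharacter snaps it to the "arme_0" socket on that character's Mesh.
; Tirer spawns an actor with the Muzzle's rotation, but its location is only that rotation's direction vector, not the muzzle position.
; It also runs a short debug-drawn Visibility line trace forward from the Muzzle, leaving the result unused.
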(event `self.Box.OnComponentBeginOverlap`
  (params (OverlappedComponent :type "PrimitiveComponent Object Reference") (OtherActor :type "Actor Object Reference") (OtherComp :type "PrimitiveComponent Object Reference") (OtherBodyIndex :type Integer) (bFromSweep :type Boolean) (SweepResult :type "HitResult Structure (by ref)"))
  (bind _asbp_first_person_character (cast `/Game/FirstPerson/Blueprints/BP_FirstPersonCharacter` OtherActor))
  (`self.K2_AttachToComponent` (`Character.Mesh` _asbp_first_person_character) "arme_0" "SnapToTarget" "SnapToTarget" "SnapToTarget"))

(fn `tirer`
  (bind _muzzle (`self.Muzzle`))
  (bind _returnvalue (`SceneComponent.K2_GetComponentLocation` _muzzle))
  (bind _returnvalue_2 (`SceneComponent.K2_GetComponentRotation` (`self.Muzzle`)))
  (`|SpawnActorFromClass` "/Game/Fab/9mm_Luger_Ammo/9mm_luger_fbx/BP_Balle.BP_Balle_C" (`KismetMathLibrary.MakeTransform` (`KismetMathLibrary.Conv_RotatorToVector` _returnvalue_2) _returnvalue_2 (5.0 5.0 5.0)) "Undefined" "MultiplyWithRoot" null null)
  (`KismetSystemLibrary.LineTraceSingle` :`Start` _returnvalue :`End` (+ (* (`SceneComponent.GetForwardVector` _muzzle) (500.0 500.0 500.0)) _returnvalue) :`TraceChannel` "TraceTypeQuery1" :`DrawDebugType` "ForDuration" :`DrawTime` 50.0))

(fn `UserConstructionScript`)